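; BP_Pick is a pickup actor, apparently a base for interactable items that can be collected, equipped or consumed.
; Its Interact event switches on PickUpType, prints a debug string, then calls Collect, Equip or Consume, passing the interacting Actor to the latter two.
; All three handlers are empty here, leaving the actual pickup behavior to be implemented, likely in child Blueprints.
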(event `/Game/Game/Blueprint/BPI_Interface/BPI_interactable.Interact`
  (params (Actor :type "Actor Object Reference"))
  (switch `/Game/Game/Blueprint/BPI_Interface/EPickUpType` (`self.PickUpType`)
    (:`NewEnumerator0`
      (`KismetSystemLibrary.PrintString` "Collerct")
      (`self.Collect`))
    (:`NewEnumerator1`
      (`KismetSystemLibrary.PrintString` "Equip")
      (`self.Equip` Actor))
    (:`NewEnumerator2`
      (`KismetSystemLibrary.PrintString` "Consume")
      (`self.Consume` Actor))))

(event `Consume`
  (params (Actor :type "Actor Object Reference")))

(event `Equip`
  (params (Actor :type "Actor Object Reference")))

(fn `Collect`)

(fn `UserConstructionScript`
  (`parent.UserConstructionScript`))